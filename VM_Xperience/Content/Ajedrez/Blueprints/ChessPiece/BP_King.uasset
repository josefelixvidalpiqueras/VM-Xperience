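; BP_King is the king piece of a chess game, providing helpers for its move highlighting and castling evaluation.
; HighlightKingSquare offsets the current position and highlights the square if IsValidMoveForKing finds it valid and free of friendly pieces, using occupancy data from the game mode.
; EvaluateCastlePath steps along Y through empty squares toward an unmoved rook at the edge, but its final rook check triggers no action yet.
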(fn `EvaluateCastlePath`
  (params (YIncrem :type Integer))
  (locals (CanContinue :type Boolean) (IsPositive :type Boolean) (TempY :type Integer))
  (bind (_chesspiece _isoccupied) (`/Game/Ajedrez/Blueprints/BP_GameMode.GetOccupant` (`self.GameModeRef`) (`self.X`) (`local.TempY`) (`self.Color`)))
  (bind (_asbp_rook _bsuccess) (cast `/Game/Ajedrez/Blueprints/ChessPiece/BP_Rook` _chesspiece :!pure true))
  (set `local.IsPositive` (> YIncrem 0))
  (set `local.TempY` (`self.Y`))
  (set `local.CanContinue` true)
  (while (`local.CanContinue`)
    (set `local.TempY` (+ YIncrem (`local.TempY`)))
    (if (and (< (`local.TempY`) 8) (> (`local.TempY`) 1))
      (set `local.CanContinue` (not (`.IsOccupied` (`/Game/Ajedrez/Blueprints/BP_GameMode.GetOccupant` (`self.GameModeRef`) (`self.X`) (`local.TempY`) (`self.Color`)))))
      (elif (and _bsuccess _isoccupied)
        (if (`/Game/Ajedrez/Blueprints/ChessPiece/BP_ChessPiece.IsInitialMove` _asbp_rook)
          _)
        (else
          (set `local.CanContinue` false))))))

(fn `HighlightKingSquare`
  (params (XIncrem :type Integer) (YIncrem :type Integer))
  (locals (TempX :type Integer) (TempY :type Integer))
  (set `local.TempX` (+ (`self.X`) XIncrem))
  (set `local.TempY` (+ (`self.Y`) YIncrem))
  (if (`self.IsValidMoveForKing` (`local.TempX`) (`local.TempY`))
    (`self.HighlightPotentialSquare` (`local.TempX`) (`local.TempY`) (`self.Color`))))

(fn `IsValidMoveForKing`
  (params (X :type Integer) (Y :type Integer))
  (returns (IsValidMove :type Boolean))
  (bind (_chesspiece _isoccupied _isoccupiedbyfriend _isvalid) (`/Game/Ajedrez/Blueprints/BP_GameMode.GetOccupant` (`self.GameModeRef`) X Y (`self.Color`)))
  (if _isvalid
    (if _isoccupiedbyfriend
      (return false)
      (else
        (return true)))
    (else
      (return false))))

(fn `UserConstructionScript`
  (`parent.UserConstructionScript`))