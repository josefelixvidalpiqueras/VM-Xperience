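; Player Blueprint for a chess game that positions the camera for the White or Black side.
; SetPlayerCamera eases the Azimuth component back to its default relative transform while moving the Camera to the White or Black component's relative transform, using MoveComponentTo.
; Despite its name, RotateCamera shifts Azimuth's relative Z location by the axis input rather than rotating it.
; Initialize and the construction script are empty.
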(event `SetPlayerCamera`
  (params (Color :type "/Game/Ajedrez/Blueprints/EN_Color Enum" :default "NewEnumerator0"))
  (bind (_returnvalue_location _returnvalue_rotation) (`KismetMathLibrary.BreakTransform` (`SceneComponent.GetRelativeTransform` (`self.Black`))))
  (bind (_returnvalue_location_2 _returnvalue_rotation_2) (`KismetMathLibrary.BreakTransform` (`SceneComponent.GetRelativeTransform` (`self.White`))))
  (`KismetSystemLibrary.MoveComponentTo` (`self.Azimuth`) (0.0 0.0 0.0) (struct) true true 1.0 true)
  (switch `/Game/Ajedrez/Blueprints/EN_Color` Color
    (:`NewEnumerator0`
      (`KismetSystemLibrary.MoveComponentTo` (`self.Camera`) _returnvalue_location_2 _returnvalue_rotation_2 true true 3.0 true))
    (:`NewEnumerator1`
      (`KismetSystemLibrary.MoveComponentTo` (`self.Camera`) _returnvalue_location _returnvalue_rotation true true 3.0 true))))

(fn `Initialize`)

(fn `RotateCamera`
  (params (Axis :type "Float (double-precision)"))
  (bind (_relativelocation_x _relativelocation_y _relativelocation_z) (`KismetMathLibrary.BreakVector` (`SceneComponent.RelativeLocation` (`self.Azimuth`))))
  (if (!= Axis 0.0)
    (`SceneComponent.K2_SetRelativeLocation` (`self.Azimuth`) (`KismetMathLibrary.MakeVector` 0.0 0.0 (+ Axis _relativelocation_z)) false false)))

(fn `UserConstructionScript`)